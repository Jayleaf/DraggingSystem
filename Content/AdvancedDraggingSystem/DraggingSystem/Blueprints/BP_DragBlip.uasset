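; BP_DragBlip is the drag target actor that carries an object grabbed by a DraggingComponent at a clamped distance before the camera.
; A looping timer interpolates blip, object and PhysicsHandle target toward that point, calling Release when the player gets too far away.
; Interpolation slows with object mass to fake weight, and a box trace can block movement on collision.
; Rotation mode applies yaw and roll input through the blip's sphere.
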(event Custom|Initialize%20Blip
  (bind _sphere (Variables|Default|GetSphere))
  (bind _returnvalue (Transformation|GetWorldRotation _sphere))
  ;[1 0.401 0.401] Set object distance from the camera on initial pickup, clamping it between the proper values.
  (bind _asdragging_component (Utilities|Casting|CastToDraggingComponent (Variables|Default|GetCaller)))
  (Variables|Default|SetObject%20Distance (Math|Float|Clamp(Float) (Transformation|GetDistanceTo self (Components|GetOwner _asdragging_component)) 3e+02 7.5e+02))
  ;[0.008445 1 0.4764] Sets interpolation speed, then begins the update timer.
  (bind _asdragging_component_2 (Utilities|Casting|CastToDraggingComponent (Variables|Default|GetCaller)))
  (CallFunction|SetInterpSpeed(Mass) _asdragging_component_2)
  (bind _returnvalue_2 (Utilities|Time|SetTimerbyEvent (delegate Custom|Blip%20Update) 0.001 true))
  (Variables|Default|SetTimer _returnvalue_2)
  ;[1 0.3543 0.5464] Grabs the object.
  (bind _asdragging_component_3 (Utilities|Casting|CastToDraggingComponent (Variables|Default|GetCaller)))
  (Physics|Components|PhysicsHandle|GrabComponentatLocationwithRotation (Variables|Default|GetPhysicsHandle) (Variables|/Game/AdvancedDraggingSystem/DraggingSystem/Components/DraggingComponent.DraggingComponent_C|Getobject _asdragging_component_3) "None" (Transformation|GetActorLocation) (Math|Interpolation|RInterpTo (Math|Rotator|MakeRotator (.roll _returnvalue) (.pitch _returnvalue) (.yaw _returnvalue)) (Math|Rotator|MakeRotator (.roll _returnvalue) (.pitch _returnvalue) (.yaw (Transformation|GetWorldRotation (Variables|/Game/AdvancedDraggingSystem/DraggingSystem/Components/DraggingComponent.DraggingComponent_C|GetCamera (.AsDragging%20Component (Utilities|Casting|CastToDraggingComponent (Variables|Default|GetCaller))))))) (Utilities|Time|GetWorldDeltaSeconds) (Variables|Default|GetInterp%20Speed)))
  (Collision|SetCollisionProfileName (Variables|/Game/AdvancedDraggingSystem/DraggingSystem/Components/DraggingComponent.DraggingComponent_C|Getobject _asdragging_component_3) "PhysicsActor" true :!class /Script/Engine.PrimitiveComponent))

(event Custom|Blip%20Update
  ;[1 0.3417 0.3915] Updates the location and rotation of the object, and will also check for distance. The distance modifier (in the > node) can be changed.
  (CallFunction|UpdateBlipLocationandRotation)
  (if (> (Transformation|GetDistanceTo (Components|GetOwner (Variables|Default|GetCamera)) self) 9e+02)
    (bind _asdragging_component (Utilities|Casting|CastToDraggingComponent (Variables|Default|GetCaller)))
    (Default|Release _asdragging_component)))

(event Custom|Deinitialize%20Blip
  ;[0.4417 0.8694 1] Blip deinitialization, which is basically just clearing the updates.
  (Utilities|Time|ClearandInvalidateTimerbyHandle (Variables|Default|GetTimer))
  (Variables|Default|SetCaller 0))

(event Custom|Enable%20Rotation%20Mode
  ;[0.08653 1 0.329] Setters for rotation mode.
  (Variables|Default|SetRotation%20Mode? true))

(event Custom|Disable%20Rotation%20Mode
  ;[0.08653 1 0.329] Setters for rotation mode.
  (Variables|Default|SetRotation%20Mode? false))

(event Custom|Change%20Roll%20Rotation
  (params (Axis%20Value :type Float%20%28single-precision%29))
  (bind _sphere (Variables|Default|GetSphere))
  (bind _returnvalue (Transformation|GetWorldRotation _sphere))
  ;[0.0245 0.8903 1] Changes the roll rotation of the object, if in rotation mode.
  (if (Variables|Default|GetRotation%20Mode?)
    (Transformation|SetWorldRotation _sphere (Math|Rotator|MakeRotator (+ (.roll _returnvalue) (* Axis%20Value 2.0)) (.pitch _returnvalue) (.yaw _returnvalue)) false false)))

(event Custom|Change%20Yaw%20Rotation
  (params (Axis%20Value :type Float%20%28single-precision%29))
  (bind _sphere (Variables|Default|GetSphere))
  (bind _returnvalue (Transformation|GetWorldRotation _sphere))
  ;[0.009047 0.9502 1] Changes the yaw rotation of the object, if in rotation mode.
  (if (Variables|Default|GetRotation%20Mode?)
    (Transformation|SetWorldRotation _sphere (Math|Rotator|MakeRotator (.roll _returnvalue) (.pitch _returnvalue) (+ (.yaw _returnvalue) (* Axis%20Value 2.0))) false false)))

(fn ConstructionScript)

(fn UpdateBlipLocationandRotation
  (bind _returnvalue (Transformation|GetActorLocation))
  (bind _sphere (Variables|Default|GetSphere))
  (bind _physicshandle (Variables|Default|GetPhysicsHandle))
  (bind _sphere_2 (Variables|Default|GetSphere))
  (bind _returnvalue_2 (Transformation|GetWorldRotation _sphere_2))
  (bind _returnvalue_3 (Transformation|GetWorldRotation _sphere))
  (bind _targetrotation (Class|PhysicsHandleComponent|GetTargetLocationandRotation _physicshandle))
  ;[1 0 0] Interpolates the blip's location to the current forward vector of the camera, and alse changes the interpolation speed based on mass. Will also check for collision. (Interpolated for smoothness)
  (bind _asdragging_component (Utilities|Casting|CastToDraggingComponent (Variables|Default|GetCaller)))
  (Variables|Default|SetCamera (Variables|/Game/AdvancedDraggingSystem/DraggingSystem/Components/DraggingComponent.DraggingComponent_C|GetCamera _asdragging_component))
  (bind _returnvalue_4 (CallFunction|CheckifColliding))
  (if _returnvalue_4
    (if (Math|Vector|NotEqual(Vector) (Variables|Default|GetMovement%20Direction) (Math|Vector|Normalize (- _returnvalue (+ (Transformation|GetWorldLocation (Variables|/Game/AdvancedDraggingSystem/DraggingSystem/Components/DraggingComponent.DraggingComponent_C|GetCamera _asdragging_component)) (* (Math|Vector|GetForwardVector (Transformation|GetWorldRotation (Variables|/Game/AdvancedDraggingSystem/DraggingSystem/Components/DraggingComponent.DraggingComponent_C|GetCamera _asdragging_component))) (Variables|Default|GetObject%20Distance))))) 1.0)
      (Transformation|SetActorLocation (Math|Interpolation|VInterpTo _returnvalue (+ (Transformation|GetWorldLocation (Variables|/Game/AdvancedDraggingSystem/DraggingSystem/Components/DraggingComponent.DraggingComponent_C|GetCamera _asdragging_component)) (* (Math|Vector|GetForwardVector (Transformation|GetWorldRotation (Variables|/Game/AdvancedDraggingSystem/DraggingSystem/Components/DraggingComponent.DraggingComponent_C|GetCamera _asdragging_component))) (Variables|Default|GetObject%20Distance))) (Utilities|Time|GetWorldDeltaSeconds) (Variables|Default|GetInterp%20Speed)) false true :!label _label)
      ;[1 0.348 0] Sets the Location of the object grabbed to the camera's forward vector
      (bind _asdragging_component_2 (Utilities|Casting|CastToDraggingComponent (Variables|Default|GetCaller)))
      (Transformation|SetWorldLocation (Variables|/Game/AdvancedDraggingSystem/DraggingSystem/Components/DraggingComponent.DraggingComponent_C|GetObject _asdragging_component_2) (Math|Interpolation|VInterpTo (Transformation|GetWorldLocation (Variables|/Game/AdvancedDraggingSystem/DraggingSystem/Components/DraggingComponent.DraggingComponent_C|GetObject _asdragging_component_2)) (+ (Transformation|GetWorldLocation (Variables|/Game/AdvancedDraggingSystem/DraggingSystem/Components/DraggingComponent.DraggingComponent_C|GetCamera _asdragging_component)) (* (Math|Vector|GetForwardVector (Transformation|GetWorldRotation (Variables|/Game/AdvancedDraggingSystem/DraggingSystem/Components/DraggingComponent.DraggingComponent_C|GetCamera _asdragging_component))) (Variables|Default|GetObject%20Distance))) (Utilities|Time|GetWorldDeltaSeconds) (Variables|Default|GetInterp%20Speed)) false false)
      ;[1 0.9826 0] Sets location and rotation of the object, again. Also accounts for rotation via rotation mode.
      (if (Variables|Default|GetRotation%20Mode?)
        (Class|PhysicsHandleComponent|SetTargetLocationandRotation (Variables|Default|GetPhysicsHandle) (Math|Interpolation|VInterpTo _returnvalue (+ (Transformation|GetWorldLocation (Variables|/Game/AdvancedDraggingSystem/DraggingSystem/Components/DraggingComponent.DraggingComponent_C|GetCamera _asdragging_component)) (* (Math|Vector|GetForwardVector (Transformation|GetWorldRotation (Variables|/Game/AdvancedDraggingSystem/DraggingSystem/Components/DraggingComponent.DraggingComponent_C|GetCamera _asdragging_component))) (Variables|Default|GetObject%20Distance))) (Utilities|Time|GetWorldDeltaSeconds) (Variables|Default|GetInterp%20Speed)) (Math|Interpolation|RInterpTo (Math|Rotator|MakeRotator (.roll _targetrotation) (.pitch _targetrotation) (.yaw _targetrotation)) (Math|Rotator|MakeRotator (.roll _returnvalue_2) (.pitch _returnvalue_2) (.yaw _returnvalue_2)) (Utilities|Time|GetWorldDeltaSeconds) (Variables|Default|GetInterp%20Speed)))
        (else
          (Class|PhysicsHandleComponent|SetTargetLocationandRotation (Variables|Default|GetPhysicsHandle) (Math|Interpolation|VInterpTo _returnvalue (+ (Transformation|GetWorldLocation (Variables|/Game/AdvancedDraggingSystem/DraggingSystem/Components/DraggingComponent.DraggingComponent_C|GetCamera _asdragging_component)) (* (Math|Vector|GetForwardVector (Transformation|GetWorldRotation (Variables|/Game/AdvancedDraggingSystem/DraggingSystem/Components/DraggingComponent.DraggingComponent_C|GetCamera _asdragging_component))) (Variables|Default|GetObject%20Distance))) (Utilities|Time|GetWorldDeltaSeconds) (Variables|Default|GetInterp%20Speed)) (Math|Interpolation|RInterpTo (Math|Rotator|MakeRotator (.roll _returnvalue_3) (.pitch _returnvalue_3) (.yaw _returnvalue_3)) (Math|Rotator|MakeRotator (.roll _returnvalue_3) (.pitch _returnvalue_3) (.yaw (Transformation|GetWorldRotation (Variables|/Game/AdvancedDraggingSystem/DraggingSystem/Components/DraggingComponent.DraggingComponent_C|GetCamera (.AsDragging%20Component (Utilities|Casting|CastToDraggingComponent (Variables|Default|GetCaller))))))) (Utilities|Time|GetWorldDeltaSeconds) (Variables|Default|GetInterp%20Speed))))))
    (else
      (goto _label))))

(fn SetInterpSpeed(Mass)
  (params (Dragging%20Component :type Dragging%20Component%20Object%20Reference))
  ;[0.6057 1 0] For each kilogram, will subtract your speed decrement divided by 600 from your interpolation speed (gives the illusion of weight)
  (for _index (range 0 (Math|Float|Round (Physics|GetMass (Variables|/Game/AdvancedDraggingSystem/DraggingSystem/Components/DraggingComponent.DraggingComponent_C|Getobject Dragging%20Component))))
    (Variables|Default|SetInterp%20Speed (Math|Float|Clamp(Float) (- (Variables|Default|GetInterp%20Speed) (/ (Variables|/Game/AdvancedDraggingSystem/DraggingSystem/Components/DraggingComponent.DraggingComponent_C|GetSpeed%20Decrement%20Per%20KG Dragging%20Component) 6e+02)) 0.01))))

(fn ResetInterpSpeed
  ;[1 1 1] Resets interp speed. Nothing much to see here. I'm just trying to comment as much as i can.
  (Variables|Default|SetInterp%20Speed 1.0))

(fn CheckifColliding
  ;[1 0.6439 0.1124] Makes a box trace around your object.
  (bind _asdragging_component (Utilities|Casting|CastToDraggingComponent (Variables|Default|GetCaller)))
  (bind (_outhit _returnvalue) (Collision|BoxTraceByChannel (.Origin (Collision|GetComponentBounds (Variables|/Game/AdvancedDraggingSystem/DraggingSystem/Components/DraggingComponent.DraggingComponent_C|Getobject _asdragging_component))) (.Origin (Collision|GetComponentBounds (Variables|/Game/AdvancedDraggingSystem/DraggingSystem/Components/DraggingComponent.DraggingComponent_C|Getobject _asdragging_component))) (.BoxExtent (Collision|GetComponentBounds (Variables|/Game/AdvancedDraggingSystem/DraggingSystem/Components/DraggingComponent.DraggingComponent_C|Getobject _asdragging_component))) "0, 0, 0" "TraceTypeQuery1" false (Utilities|Array|MakeArray self (Components|GetOwner (Variables|/Game/AdvancedDraggingSystem/DraggingSystem/Components/DraggingComponent.DraggingComponent_C|Getobject _asdragging_component)) (Components|GetOwner _asdragging_component)) "None"))
  ;[0.6977 1 0] Gets the movement direction of the object
  (Variables|Default|SetMovement%20Direction (Math|Vector|Normalize (- (.Origin (Collision|GetComponentBounds (Variables|/Game/AdvancedDraggingSystem/DraggingSystem/Components/DraggingComponent.DraggingComponent_C|Getobject _asdragging_component))) (.ImpactPoint (Collision|BreakHitResult _outhit)))))
  (return _returnvalue))